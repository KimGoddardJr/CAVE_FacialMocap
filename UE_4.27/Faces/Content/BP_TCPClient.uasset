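; Test TCP client Blueprint that connects to a local server on BeginPlay and prints what it receives.
; Connection and message callbacks print status, and each message is decoded as a full-length string and printed.
; An alternative float read and the FInput assignment, noted as meant for an AnimBP, are unwired and never run.
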(event Custom|Disconnected
  (params (ConnectionId :type Integer))
  ;[1 1 1] Comment
)

(event Custom|Connected
  (params (ConnectionId :type Integer))
  ;[1 1 1] Comment
  (if true
    (Development|PrintString "Connected")))

(event Custom|MessageRcvd
  (params (ConnectionId :type Integer) (Message :type Array%20of%20Bytes))
  ;[1 1 1] Comment
  (Development|PrintString "Message Received!")
  (bind _returnvalue (Class|TcpSocketConnection|MessageReadString Message (Utilities|Array|Length Message)))
  (Development|PrintString _returnvalue))

(event EventBeginPlay
  ;[1 1 1] TCP Connection
  (Class|TcpSocketConnection|Connect "127.0.0.1" 65432 (delegate Custom|Disconnected) (delegate Custom|Connected) (delegate Custom|MessageRcvd)))

(event EventTick
  (params (DeltaSeconds :type Float%20%28single-precision%29)))

(fn ConstructionScript)